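; Vertical zipline actor that the first-person character rides up and down along a spline.
; Overlapping the ground or top capsule allows toggling engagement with F and, while disengaged, resets travel to that end.
; While engaged, W and S change the travel distance on Tick, and the character is moved to that spline time's world location.
; Moving past either end of the range disengages the ride automatically.
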(event `self.ReceiveTick`
  (params (DeltaSeconds :type "Float (single-precision)"))
  (set `self.Delta Seconds` DeltaSeconds)
  (`self.DistanceCheck`)
  (`|ExecutionSequence`
    (:`then_0`
      (if (`self.ZipUp`)
        (set `self.Distance` (+ (`self.Distance`) (* (`self.Delta Seconds`) 1.5)))))
    (:`then_1`
      (if (`self.ZipDown`)
        (set `self.Distance` (- (`self.Distance`) (* (`self.Delta Seconds`) 1.5)))))
    (:`then_2`
      (if (`self.Engage`)
        (`self.CustomEvent`)))))

(event `self.ReceiveBeginPlay`
  (bind _returnvalue (`GameplayStatics.GetActorOfClass` "/Game/FirstPerson/Blueprints/BP_FirstPersonCharacter.BP_FirstPersonCharacter_C"))
  (set `self.BP_Character` _returnvalue))

(event `Key|W`
  (params (Key :type "Key Structure"))
  (:`Pressed`
    (if (`self.Engage`)
      (set `self.ZipUp` true)))
  (:`Released`
    (set `self.ZipUp` false)))

(event `self.GroundCapsule.OnComponentBeginOverlap`
  (params (OverlappedComponent :type "PrimitiveComponent Object Reference") (OtherActor :type "Actor Object Reference") (OtherComp :type "PrimitiveComponent Object Reference") (OtherBodyIndex :type Integer) (bFromSweep :type Boolean) (SweepResult :type "HitResult Structure (by ref)"))
  ;[1 1 1] Comment
  (if (`self.Engage`)
    (if (== OtherActor (`self.BP_Character`))
      _)
    (elif (== OtherActor (`self.BP_Character`))
      (set `self.Is Colliding` true)
      (set `self.Distance` 0.0))))

(event `Key|S`
  (params (Key :type "Key Structure"))
  (:`Pressed`
    (if (`self.Engage`)
      (set `self.ZipDown` true)))
  (:`Released`
    (set `self.ZipDown` false)))

(event `self.TopCapsule.OnComponentBeginOverlap`
  (params (OverlappedComponent :type "PrimitiveComponent Object Reference") (OtherActor :type "Actor Object Reference") (OtherComp :type "PrimitiveComponent Object Reference") (OtherBodyIndex :type Integer) (bFromSweep :type Boolean) (SweepResult :type "HitResult Structure (by ref)"))
  ;[1 0.4271 0.8866] Comment
  (if (`self.Engage`)
    (if (== OtherActor (`self.BP_Character`))
      _)
    (elif (== OtherActor (`self.BP_Character`))
      (set `self.Is Colliding` true)
      (set `self.Distance` 4.0))))

(event `Key|F`
  (params (Key :type "Key Structure"))
  (:`Pressed`
    (if (`self.Is Colliding`)
      (if (`self.Engage`)
        (set `self.Engage` false)
        (else
          (set `self.Engage` true))))))

(event `CustomEvent`
  (`self.K2_SetActorRelativeTransform` (`self.BP_Character`) (`KismetMathLibrary.Conv_VectorToTransform` (`SplineComponent.GetLocationAtTime` (`self.Spline1`) (`self.Distance`) "World" false)) false false))

(event `self.GroundCapsule.OnComponentEndOverlap`
  (params (OverlappedComponent :type "PrimitiveComponent Object Reference") (OtherActor :type "Actor Object Reference") (OtherComp :type "PrimitiveComponent Object Reference") (OtherBodyIndex :type Integer))
  ;[0.6495 1 0.5619] Comment
  (if (== OtherActor (`self.BP_Character`))
    (set `self.Is Colliding` false)))

(event `self.TopCapsule.OnComponentEndOverlap`
  (params (OverlappedComponent :type "PrimitiveComponent Object Reference") (OtherActor :type "Actor Object Reference") (OtherComp :type "PrimitiveComponent Object Reference") (OtherBodyIndex :type Integer))
  ;[0.6495 1 0.5619] Comment
  (if (== OtherActor (`self.BP_Character`))
    (set `self.Is Colliding` false)))

(fn `DistanceCheck`
  (if (or (> (`self.Distance`) 4.0) (< (`self.Distance`) 0.0))
    (set `self.Engage` false)))

(fn `UserConstructionScript`)