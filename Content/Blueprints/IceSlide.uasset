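; Ice slide actor that carries the first-person character along a spline.
; Overlapping the start collider resets progress and engages the slide; overlapping the end collider while engaged stops it.
; While engaged, Tick advances spline time at double speed and sets the character's relative transform from that world-space spline location.
; An unconnected debug-printing block holds a manual engage toggle.
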(event `self.ReceiveTick`
  (params (DeltaSeconds :type "Float (single-precision)"))
  (set `self.Delta Seconds` DeltaSeconds)
  (`|ExecutionSequence`
    (:`then_0`
      (if (`self.Engage`)
        (set `self.Distance` (+ (`self.Distance`) (* (`self.Delta Seconds`) 2.0)))))
    (:`then_2`
      (if (`self.Engage`)
        (`self.CustomEvent`)))))

(event `self.ReceiveBeginPlay`
  (bind _returnvalue (`GameplayStatics.GetActorOfClass` "/Game/FirstPerson/Blueprints/BP_FirstPersonCharacter.BP_FirstPersonCharacter_C"))
  (set `self.BP_Character` _returnvalue))

(event `self.Start Collider.OnComponentBeginOverlap`
  (params (OverlappedComponent :type "PrimitiveComponent Object Reference") (OtherActor :type "Actor Object Reference") (OtherComp :type "PrimitiveComponent Object Reference") (OtherBodyIndex :type Integer) (bFromSweep :type Boolean) (SweepResult :type "HitResult Structure (by ref)"))
  ;[1 1 1] Comment
  (if (`self.Engage`)
    (if (== OtherActor (`self.BP_Character`))
      _)
    (elif (== OtherActor (`self.BP_Character`))
      (set `self.Is Colliding` true)
      (set `self.Distance` 0.0)
      (set `self.Engage` true))))

(event `self.End Collider.OnComponentBeginOverlap`
  (params (OverlappedComponent :type "PrimitiveComponent Object Reference") (OtherActor :type "Actor Object Reference") (OtherComp :type "PrimitiveComponent Object Reference") (OtherBodyIndex :type Integer) (bFromSweep :type Boolean) (SweepResult :type "HitResult Structure (by ref)"))
  ;[1 0.4271 0.8866] Comment
  (if (`self.Engage`)
    (if (== OtherActor (`self.BP_Character`))
      (set `self.Engage` false))
    (elif (== OtherActor (`self.BP_Character`))
      (set `self.Is Colliding` true)
      (set `self.Distance` 4.0))))

(event `Key|F`
  (params (Key :type "Key Structure")))

(event `CustomEvent`
  (`self.K2_SetActorRelativeTransform` (`self.BP_Character`) (`KismetMathLibrary.Conv_VectorToTransform` (`SplineComponent.GetLocationAtTime` (`self.Spline`) (`self.Distance`) "World" false)) false false))

(event `self.Start Collider.OnComponentEndOverlap`
  (params (OverlappedComponent :type "PrimitiveComponent Object Reference") (OtherActor :type "Actor Object Reference") (OtherComp :type "PrimitiveComponent Object Reference") (OtherBodyIndex :type Integer))
  (if (== OtherActor (`self.BP_Character`))
    (set `self.Is Colliding` false)))

(event `self.End Collider.OnComponentEndOverlap`
  (params (OverlappedComponent :type "PrimitiveComponent Object Reference") (OtherActor :type "Actor Object Reference") (OtherComp :type "PrimitiveComponent Object Reference") (OtherBodyIndex :type Integer))
  (if (== OtherActor (`self.BP_Character`))
    (set `self.Is Colliding` false)))

(fn `UserConstructionScript`)